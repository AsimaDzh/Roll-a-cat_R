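; Game mode for the cat game that tracks collected items, shows the count on a HUD widget and handles winning.
; BeginPlay creates the HUD and resets the count, and each Update call increments it and refreshes the widget.
; Once the count reaches four, it waits briefly, plays a level-complete sound, shows the win screen and pauses the game.
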(event `self.ReceiveBeginPlay`
  (bind _returnvalue (`|CreateWidget` "/Game/Blueprints/Widjets/Widgets.Widgets_C"))
  (bind _output_get (set `self.UI` _returnvalue))
  (`UserWidget.AddToViewport` _output_get 0)
  (`self.Reset`))

(event `Reset`
  (set `self.Items` 0)
  (set `/Game/Blueprints/Widjets/Widgets.Point` 0 (`self.UI`)))

(event `Update`
  (bind _output_get (set `self.Items` (+ 1 (`self.Items`))))
  (set `/Game/Blueprints/Widjets/Widgets.Point` _output_get (`self.UI`))
  (`self.End Game`))

(event `End Game`
  (if (>= (`self.Items`) 4)
    (`KismetSystemLibrary.Delay` 0.5)
    (`GameplayStatics.SpawnSound2D` "/Game/Blueprints/Sounds/Level_Complete.Level_Complete" 1.0 1.0 0.0 null)
    (bind _returnvalue (`|CreateWidget` "/Game/Blueprints/Widjets/You_Win_W.You_Win_W_C"))
    (bind _output_get (set `self.You Win` _returnvalue))
    (`UserWidget.AddToViewport` _output_get 0)
    (`GameplayStatics.SetGamePaused` true)))

(fn `UserConstructionScript`)