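; Cat controller that tracks the six food pickups the cat finds and unlocks level 2 once all are found.
; On BeginPlay it adds a pickup icon widget to the viewport.
; Each Found event forwards to a Client counterpart that updates the widget, increments a shared counter and plays its own meow.
; At six, the widget shows completion and a newly created SaveLevel object with Level2Unlocked is written to Slot1.
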(event `self.ReceiveBeginPlay`
  (bind _returnvalue (`|CreateWidget` "/Game/Blueprints/Widjets/Pickup_Icons_W.Pickup_Icons_W_C"))
  (bind _output_get (set `self.Pickup Icons` _returnvalue))
  (`UserWidget.AddToViewport` _output_get 0))

(event `Client Found Cake`
  (bind _pickup_icons (`self.Pickup Icons`))
  (bind _found_all (`self.Found all`))
  (`/Game/Blueprints/Widjets/Pickup_Icons_W.Found Cake` _pickup_icons)
  (`/Engine/EditorBlueprintResources/StandardMacros.IncrementInt` _found_all
    (:`  `
      (`GameplayStatics.PlaySound2D` "/Game/Blueprints/Sounds/meow1.meow1" 1.0 1.0 0.0 null null)
      (if (== _found_all 6) :!label _label
        (`/Game/Blueprints/Widjets/Pickup_Icons_W.Found all` _pickup_icons)
        (bind _returnvalue (`GameplayStatics.CreateSaveGameObject` "/Game/Blueprints/Levels/SaveLevel.SaveLevel_C"))
        (set `/Game/Blueprints/Levels/SaveLevel.Level2 Unlocked` true _returnvalue)
        (`GameplayStatics.SaveGameToSlot` _returnvalue "Slot1")))))

(event `/Game/Blueprints/Pickup/BP_Interface_Controller.Found_Cake`
  (`self.Client Found Cake`))

(event `Client Found Cupcake`
  (`/Game/Blueprints/Widjets/Pickup_Icons_W.Found Cupcake` (`self.Pickup Icons`))
  (`/Engine/EditorBlueprintResources/StandardMacros.IncrementInt` (`self.Found all`)
    (:`  `
      (`GameplayStatics.PlaySound2D` "/Game/Blueprints/Sounds/meow2.meow2" 1.0 1.0 0.0 null null)
      (goto _label))))

(event `/Game/Blueprints/Pickup/BP_Interface_Controller.Found_Cupcake`
  (`self.Client Found Cupcake`))

(event `Client Found Icecream`
  (`/Game/Blueprints/Widjets/Pickup_Icons_W.Found Icecream` (`self.Pickup Icons`))
  (`/Engine/EditorBlueprintResources/StandardMacros.IncrementInt` (`self.Found all`)
    (:`  `
      (`GameplayStatics.PlaySound2D` "/Game/Blueprints/Sounds/meow3.meow3" 1.0 1.0 0.0 null null)
      (goto _label))))

(event `/Game/Blueprints/Pickup/BP_Interface_Controller.Found_Icecream`
  (`self.Client Found Icecream`))

(event `Client Found Milkshake`
  (`/Game/Blueprints/Widjets/Pickup_Icons_W.Found Milkshake` (`self.Pickup Icons`))
  (`/Engine/EditorBlueprintResources/StandardMacros.IncrementInt` (`self.Found all`)
    (:`  `
      (`GameplayStatics.PlaySound2D` "/Game/Blueprints/Sounds/meow4.meow4" 1.0 1.0 0.0 null null)
      (goto _label))))

(event `/Game/Blueprints/Pickup/BP_Interface_Controller.Found_Milkshake`
  (`self.Client Found Milkshake`))

(event `/Game/Blueprints/Pickup/BP_Interface_Controller.Found_Cheese`
  (`self.Client Found Cheese`))

(event `Client Found Cheese`
  (`/Game/Blueprints/Widjets/Pickup_Icons_W.Found cheese` (`self.Pickup Icons`))
  (`/Engine/EditorBlueprintResources/StandardMacros.IncrementInt` (`self.Found all`)
    (:`  `
      (`GameplayStatics.PlaySound2D` "/Game/Blueprints/Sounds/angry_meow.angry_meow" 1.0 1.0 0.0 null null)
      (goto _label))))

(event `Client Found Cucumber`
  (`/Game/Blueprints/Widjets/Pickup_Icons_W.Found cucumber` (`self.Pickup Icons`))
  (`/Engine/EditorBlueprintResources/StandardMacros.IncrementInt` (`self.Found all`)
    (:`  `
      (`GameplayStatics.PlaySound2D` "/Game/Blueprints/Sounds/surprised_meow.surprised_meow" 1.0 1.0 0.0 null null)
      (goto _label))))

(event `/Game/Blueprints/Pickup/BP_Interface_Controller.Found_Cucumber`
  (`self.Client Found Cucumber`))

(fn `UserConstructionScript`)