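; BP_Base is a spinning food pickup that actors tagged "Cat" collect by overlapping its sphere.
; On authority, the overlap spawns a coin-burst effect, removes the pickup and sphere components, then destroys the actor.
; The Cake value selects which food-found message, from cake to cucumber, goes to the collector's instigator controller.
; Tick rotates the actor on all three axes at a rate set by Speed.
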(event `self.Sphere.OnComponentBeginOverlap`
  (params (OverlappedComponent :type "PrimitiveComponent Object Reference") (OtherActor :type "Actor Object Reference") (OtherComp :type "PrimitiveComponent Object Reference") (OtherBodyIndex :type Integer) (bFromSweep :type Boolean) (SweepResult :type "HitResult Structure (by ref)"))
  (bind _returnvalue (`self.GetInstigatorController` OtherActor))
  (`/Engine/EditorBlueprintResources/ActorMacros.Switch Has Authority`
    (:`Authority`
      (if (`self.ActorHasTag` OtherActor "Cat")
        (`NiagaraFunctionLibrary.SpawnSystemAtLocation` "/Game/Blueprints/Pickup/Coins_Explode.Coins_Explode" (`self.K2_GetActorLocation`) (struct) (1.0 1.0 1.0) true true "AutoRelease")
        (`ActorComponent.K2_DestroyComponent` (`self.Pickup`))
        (`ActorComponent.K2_DestroyComponent` (`self.Sphere`))
        (switch `int` (`self.Cake`)
          (:`0`
            (message `/Game/Blueprints/Pickup/BP_Interface_Controller.Found_Cake` _returnvalue))
          (:`1`
            (message `/Game/Blueprints/Pickup/BP_Interface_Controller.Found_Cupcake` _returnvalue))
          (:`2`
            (message `/Game/Blueprints/Pickup/BP_Interface_Controller.Found_Icecream` _returnvalue))
          (:`3`
            (message `/Game/Blueprints/Pickup/BP_Interface_Controller.Found_Milkshake` _returnvalue))
          (:`4`
            (message `/Game/Blueprints/Pickup/BP_Interface_Controller.Found_Cheese` _returnvalue))
          (:`5`
            (message `/Game/Blueprints/Pickup/BP_Interface_Controller.Found_Cucumber` _returnvalue)))
        (`self.K2_DestroyActor`)))))

(event `self.ReceiveTick`
  (params (DeltaSeconds :type "Float (single-precision)"))
  (bind _speed (`self.Speed`))
  (`self.K2_AddActorLocalRotation` (* (`KismetMathLibrary.MakeRotator` _speed _speed _speed) DeltaSeconds)))

(fn `UserConstructionScript`)