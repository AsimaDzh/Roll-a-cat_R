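; BP_Juice is a spinning pickup that the cat collects by touching it.
; Each tick it rotates on all three local axes at a rate set by Speed.
; When BP_Cat overlaps its sphere, it plays a meow, spawns a pooled Niagara coin burst and destroys itself, then calls Update on BP_Cat_GameMode to register the pickup.
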(event `self.Sphere.OnComponentBeginOverlap`
  (params (OverlappedComponent :type "PrimitiveComponent Object Reference") (OtherActor :type "Actor Object Reference") (OtherComp :type "PrimitiveComponent Object Reference") (OtherBodyIndex :type Integer) (bFromSweep :type Boolean) (SweepResult :type "HitResult Structure (by ref)"))
  (bind _returnvalue (`self.K2_GetActorLocation`))
  (cast `/Game/Blueprints/Cat/BP_Cat` OtherActor)
  (`GameplayStatics.PlaySoundAtLocation` "/Game/Blueprints/Sounds/meow4.meow4" _returnvalue (struct) 1.0 1.0 0.0 null null null null)
  (`NiagaraFunctionLibrary.SpawnSystemAtLocation` "/Game/Blueprints/Pickup/Coins_Explode.Coins_Explode" _returnvalue (struct) (1.0 1.0 1.0) true true "AutoRelease")
  (`self.K2_DestroyActor`)
  (bind _asbp_cat_game_mode (cast `/Game/Blueprints/Cat/BP_Cat_GameMode` (`GameplayStatics.GetGameMode`)))
  (`/Game/Blueprints/Cat/BP_Cat_GameMode.Update` _asbp_cat_game_mode))

(event `self.ReceiveTick`
  (params (DeltaSeconds :type "Float (single-precision)"))
  (bind _speed (`self.Speed`))
  (`self.K2_AddActorLocalRotation` (* (`KismetMathLibrary.MakeRotator` _speed _speed _speed) DeltaSeconds)))

(fn `UserConstructionScript`)